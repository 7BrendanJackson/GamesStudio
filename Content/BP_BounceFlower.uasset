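; BP_BounceFlower is a bounce pad that launches the player character upward when it touches the flower.
; Activate and Deactivate events toggle an On flag that gates the bounce.
; When the Box begins overlapping a BP_RegrowthCharacter while On, LaunchCharacter applies world up times Force, overriding vertical velocity but keeping horizontal momentum.
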(event OnComponentBeginOverlap(Box)
  (params (OverlappedComponent :type Primitive%20Component%20Object%20Reference) (OtherActor :type Actor%20Object%20Reference) (OtherComp :type Primitive%20Component%20Object%20Reference) (OtherBodyIndex :type Integer) (bFromSweep :type Boolean) (SweepResult :type Hit%20Result%20Structure%20%28by%20ref%29))
  (bind _asbp_regrowth_character (Utilities|Casting|CastToBP_RegrowthCharacter OtherActor))
  (if (Variables|Default|Geton?)
    (Character|LaunchCharacter _asbp_regrowth_character (* (Math|Vector|VectorUp) (Variables|Default|GetForce)) false true)))

(event EventActivate
  (Variables|Default|Seton? true))

(event EventDeactivate
  (Variables|Default|Seton? false))

(fn ConstructionScript)