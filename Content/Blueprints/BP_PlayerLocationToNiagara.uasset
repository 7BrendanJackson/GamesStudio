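; Trigger actor that steers a referenced Niagara system's User.PlayerLocation toward the player while inside its volume.
; Begin and end overlaps with BP_RegrowthCharacter toggle FollowPlayer.
; While following, a Delay on Tick throttles updates to roughly half-second steps, sending the Character's location plus a random horizontal offset.
; Construction, BeginPlay and trigger exit set the parameter to the Niagara actor's own location.
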(event OnComponentEndOverlap(Trigger)
  (params (OverlappedComponent :type Primitive%20Component%20Object%20Reference) (OtherActor :type Actor%20Object%20Reference) (OtherComp :type Primitive%20Component%20Object%20Reference) (OtherBodyIndex :type Integer))
  (bind _niagarasystem (Variables|Default|GetNiagaraSystem))
  (Utilities|Casting|CastToBP_RegrowthCharacter OtherActor)
  (Variables|Default|SetFollowPlayer false)
  (Niagara|SetNiagaraVariable(Vector3) (Variables|/Script/Niagara.NiagaraActor|GetNiagaraComponent _niagarasystem) "User.PlayerLocation" (Transformation|GetActorLocation _niagarasystem)))

(event OnComponentBeginOverlap(Trigger)
  (params (OverlappedComponent :type Primitive%20Component%20Object%20Reference) (OtherActor :type Actor%20Object%20Reference) (OtherComp :type Primitive%20Component%20Object%20Reference) (OtherBodyIndex :type Integer) (bFromSweep :type Boolean) (SweepResult :type Hit%20Result%20Structure%20%28by%20ref%29))
  (Utilities|Casting|CastToBP_RegrowthCharacter OtherActor)
  (Variables|Default|SetFollowPlayer true))

(event EventTick
  (params (DeltaSeconds :type Float%20%28single-precision%29))
  (bind _returnvalue (Math|Random|RandomUnitVector))
  (bind _returnvalue_2 (Math|Vector|MakeVector (.x _returnvalue) (.y _returnvalue) 0.0))
  (bind _returnvalue_3 (Math|Vector|Normalize _returnvalue_2))
  (if (Variables|Default|GetFollowPlayer)
    (Utilities|FlowControl|Delay 0.5)
    (Niagara|SetNiagaraVariable(Vector3) (Variables|/Script/Niagara.NiagaraActor|GetNiagaraComponent (Variables|Default|GetNiagaraSystem)) "User.PlayerLocation" (+ (Transformation|GetActorLocation (Variables|Default|GetCharacter)) (Math|Vector|MakeVector (* (.x _returnvalue_3) 1e+02) (* (.y _returnvalue_3) 1e+02) 0.0)))))

(event EventBeginPlay
  (bind _niagarasystem (Variables|Default|GetNiagaraSystem))
  (Niagara|SetNiagaraVariable(Vector3) (Variables|/Script/Niagara.NiagaraActor|GetNiagaraComponent _niagarasystem) "User.PlayerLocation" (Transformation|GetActorLocation _niagarasystem)))

(fn ConstructionScript
  (bind _niagarasystem (Variables|Default|GetNiagaraSystem))
  (Niagara|SetNiagaraVariable(Vector3) (Variables|/Script/Niagara.NiagaraActor|GetNiagaraComponent _niagarasystem) "User.PlayerLocation" (Transformation|GetActorLocation _niagarasystem)))