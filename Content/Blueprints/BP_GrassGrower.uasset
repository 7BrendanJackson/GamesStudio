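; BP_GrassGrower is an actor that displays how many vertices of its static mesh have green vertex paint.
; Tick, throttled by a one-second Delay, and the painted-at-location event both request all vertex colors through the Runtime Vertex Paint and Detection component.
; The result callback counts LOD 0 vertices with nonzero green and writes that number to a TextRender.
; Only the Tick request explicitly includes per-vertex color data.
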(event GetAllVertexColorsOnlyDelegate(BPC_RuntimeVertexPaintAndDetectionComponent)
  (params (taskResultInfo :type Vertex%20Detect%20Task%20Result%20Info%20Structure) (meshVertexData :type Vertex%20Detect%20Mesh%20Data%20Struct%20Structure) (gotAllVertexColorsWithSettings :type Vertex%20Detect%20Get%20Colors%20Only%20Struct%20Structure) (amountOfPaintedColorsOfEachChannel :type Vertex%20Detect%20Amount%20Of%20Painted%20Colors%20Of%20Each%20Channel%20Structure) (vertexColorsOnEachBone :type Vertex%20Detect%20Vertex%20Colors%20on%20Each%20Bone%20Structure) (additionalData :type Vertex%20Detect%20Additional%20Data%20to%20Pass%20Through%20Structure))
  (Variables|Default|SetGreenCount 0)
  (for _array_element (.meshVertexColorsPerLODArray (Utilities|Struct|BreakVertexDetectMeshDataPerLODStruct (Utilities|Array|Get(acopy) (.meshDataPerLOD (Utilities|Struct|BreakVertexDetectMeshDataStruct meshVertexData)))))
    (if (> (.g _array_element) 0)
      (Math|Integer|IncrementInt (Variables|Default|GetGreenCount))))
  (Rendering|Components|TextRender|SetText (Variables|Default|GetTextRender) (Utilities|Text|ToText(Integer) (Variables|Default|GetGreenCount))))

(event VertexColorsPaintedatLocationDelegate(BPC_RuntimeVertexPaintAndDetectionComponent)
  (params (taskResultInfo :type Vertex%20Detect%20Task%20Result%20Info%20Structure) (meshVertexData :type Vertex%20Detect%20Mesh%20Data%20Struct%20Structure) (meshPaintedWithSettings :type Vertex%20Paint%20at%20Location%20Struct%20Structure) (closestVertexInfoAfterApplyingColor :type Vertex%20Detect%20Closest%20Vertex%20Data%20Result%20Struct%20Structure) (estimatedColorAtHitLocationInfo :type Vertex%20Detect%20Estimated%20Color%20at%20Hit%20Location%20Result%20Struct%20Structure) (avarageColorInAreaInfo :type Vertex%20Detect%20Avarage%20Color%20in%20Area%20Info%20Structure) (amountOfPaintedColorsOfEachChannel :type Vertex%20Detect%20Amount%20Of%20Painted%20Colors%20Of%20Each%20Channel%20Structure) (vertexColorsOnEachBone :type Vertex%20Detect%20Vertex%20Colors%20on%20Each%20Bone%20Structure) (additionalData :type Vertex%20Detect%20Additional%20Data%20to%20Pass%20Through%20Structure))
  (|GetAllVertexColorsOnlyNode (Variables|Default|GetBPC_RuntimeVertexPaintAndDetectionComponent) (Variables|Debug|GetStaticMeshComponent) (Utilities|Struct|MakeVertexDetectGetColorsOnlyStruct (Utilities|Struct|MakeVertexDetectEventSettings true true true false (Utilities|Struct|MakeVertexDetectIncludeAmountOfPaintedColorsOfEachChannel true 0.5)) "(useMultithreadingForCalculations=True,multithreadPriority=TPri_Highest)")))

(event EventTick
  (params (DeltaSeconds :type Float%20%28single-precision%29))
  (Utilities|FlowControl|Delay 1.0)
  (|GetAllVertexColorsOnlyNode (Variables|Default|GetBPC_RuntimeVertexPaintAndDetectionComponent) (Variables|Debug|GetStaticMeshComponent) (Utilities|Struct|MakeVertexDetectGetColorsOnlyStruct (Utilities|Struct|MakeVertexDetectEventSettings true true true false (Utilities|Struct|MakeVertexDetectIncludeAmountOfPaintedColorsOfEachChannel true 0.5) true) "(useMultithreadingForCalculations=True,multithreadPriority=TPri_Highest)")))

(fn ConstructionScript)