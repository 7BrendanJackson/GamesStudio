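; Paintable canvas actor that stamps a brush texture where the player's camera is aimed on each left mouse click.
; BeginPlay creates and clears a render target, feeds it into a dynamic canvas material, and creates a dynamic brush material.
; A click line-traces from the camera, ignoring BP_RegrowthCharacter actors, and converts a canvas hit to UVs via FindCollisionUV.
; DrawBrush then draws the brush material into the render target, centered on that UV.
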(event EventBeginPlay
  (Utilities|FlowControl|Sequence
    (:then_0
      (bind _returnvalue (Rendering|CreateRenderTarget2D 1024 1024 "RTF_RGBA16f"))
      (bind _output_get (Variables|Default|SetRenderTarget _returnvalue))
      (Rendering|ClearRenderTarget2D _output_get "(R=0.070000,G=0.130000,B=0.060000,A=1.000000)"))
    (:then_1
      (bind _returnvalue_2 (Rendering|Material|CreateDynamicMaterialInstance "/Game/Materials/M_Canvas.M_Canvas" "None" "None" :!class /Script/Engine.KismetMaterialLibrary))
      (Rendering|Material|SetTextureParameterValue _returnvalue_2 "RenderTarget" (Variables|Default|GetRenderTarget))
      (Rendering|Material|SetMaterial (Variables|Default|GetCanvas) 0 _returnvalue_2))
    (:then_2
      (bind _returnvalue_3 (Rendering|Material|CreateDynamicMaterialInstance "/Game/Materials/M_Brush.M_Brush" "None" "None" :!class /Script/Engine.KismetMaterialLibrary))
      (Variables|Default|SetBrushMaterial _returnvalue_3))))

(event Input|MouseEvents|LeftMouseButton
  (params (Key :type Key%20Structure))
  (bind _returnvalue (Game|GetPlayerCameraManager 0))
  (bind _returnvalue_2 (Transformation|GetActorLocation _returnvalue))
  (:Pressed
    (bind _outactors (Actor|GetAllActorsOfClass "/Game/ThirdPerson/Blueprints/BP_RegrowthCharacter.BP_RegrowthCharacter_C"))
    (bind (_outhit _returnvalue_3) (Collision|LineTraceByChannel _returnvalue_2 (+ _returnvalue_2 (* (Transformation|GetActorForwardVector _returnvalue) 10000)) "TraceTypeQuery2" true _outactors "ForDuration" false))
    (Utilities|Casting|CastToBP_Canvas (.HitActor (Collision|BreakHitResult _outhit))
      (:then
        (Variables|Default|SetDrawLocation (.UV (Class|GameplayStatics|FindCollisionUV _outhit)))
        (CallFunction|DrawBrush))
      (:CastFailed
        (Development|PrintString (Utilities|String|ToString(Boolean) _returnvalue_3))))))

(fn ConstructionScript)

(fn DrawBrush
  (bind _brushsize (Variables|Default|GetBrushSize))
  (bind _returnvalue (/ _brushsize 2.0))
  (Utilities|FlowControl|Sequence
    (:then_0
      (Rendering|Material|SetTextureParameterValue (Variables|Default|GetBrushMaterial) "BrushTexture" (Variables|Default|GetBrushTexture)))
    (:then_1
      (bind (_canvas _size _context) (Rendering|BeginDrawCanvastoRenderTarget (Variables|Default|GetRenderTarget)))
      (Canvas|DrawMaterial :self _canvas :RenderMaterial (Variables|Default|GetBrushMaterial) :ScreenPosition (- (* _size (Variables|Default|GetDrawLocation)) (Math|Vector2D|MakeVector2D _returnvalue _returnvalue)) :ScreenSize (Math|Vector2D|MakeVector2D _brushsize _brushsize) :CoordinateSize "(X=1.000000,Y=1.000000)" :PivotPoint "(X=0.500000,Y=0.500000)")
      (Rendering|EndDrawCanvastoRenderTarget _context))))