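; BP_Pause is an actor that handles pausing the game and shows a pause menu widget.
; On BeginPlay it creates a BP_PauseMenu widget, adds it to the viewport and hides it.
; P or Escape toggles the paused state and sets the menu visible on every press, with no hiding on unpause here.
; The construction script also adds a widget component without assigning it a widget.
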(event EventBeginPlay
  (bind _returnvalue (UserInterface|CreateWidget "/Game/BP_PauseMenu.BP_PauseMenu_C"))
  (bind _output_get (Variables|Default|SetMenu _returnvalue))
  (UserInterface|Viewport|AddtoViewport _returnvalue 0)
  (Widget|SetVisibility _output_get "Hidden"))

(event Collision|EventActorBeginOverlap
  (params (OtherActor :type Actor%20Object%20Reference)))

(event EventTick
  (params (DeltaSeconds :type Float%20%28single-precision%29)))

(event Input|KeyboardEvents|Escape
  (params (Key :type Key%20Structure :default "None"))
  (:Pressed
    (Game|SetGamePaused (not (Game|IsGamePaused)))
    (Widget|SetVisibility (Variables|Default|GetMenu) "Visible")))

(event Input|KeyboardEvents|P
  (params (Key :type Key%20Structure :default "None"))
  (:Pressed
    (Game|SetGamePaused (not (Game|IsGamePaused)))
    (Widget|SetVisibility (Variables|Default|GetMenu) "Visible")))

(fn ConstructionScript
  (bind _returnvalue (AddComponent|AddWidgetComponent false))
  (UserInterface|SetWidget _returnvalue 0))